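; Engineer variant of the AI character that deploys Fodder characters.
; Its Shoot event spawns a BP_Character_Fodder at the ShootPoint component's world transform.
; All other behavior comes from the parent class, as the construction script only calls the parent and the default event nodes are disabled.
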(event `self.Shoot`
  (params (ProjectileClass :type "Actor Class Reference"))
  (`|SpawnActorFromClass` "/Game/Characters/AICharacter/Variants/Fodder/BP_Character_Fodder.BP_Character_Fodder_C" (`SceneComponent.K2_GetComponentToWorld` (`self.ShootPoint`)) "Undefined" "MultiplyWithRoot" null null))

(fn `UserConstructionScript`
  (`parent.UserConstructionScript`))