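; Leader variant of the AI character that topples over and breaks apart when killed.
; On VitalityComponent death it sets LeaderIsDead on its controller's blackboard and lets the capsule simulate physics.
; A looping timer watches the capsule's up vector until it has tipped far enough, then detaches the body meshes as physics pieces, disables the capsule and unpossesses the controller.
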(event `self.VitalityComponent.Death`
  (`BlackboardComponent.SetValueAsBool` (`AIBlueprintHelperLibrary.GetBlackboard` (`self.GetController`)) (`self.LeaderIsDead`) true)
  (`PrimitiveComponent.SetSimulatePhysics` (`self.CapsuleComponent`) true)
  (bind _returnvalue (`KismetSystemLibrary.K2_SetTimerDelegate` (delegate `ToppelTimerCB`) 0.3 true))
  (set `self.ToppleTimer` _returnvalue))

(event `ToppelTimerCB`
  (bind _returnvalue (`self.GetController`))
  (if (< (.z (`SceneComponent.GetUpVector` (`self.CapsuleComponent`))) 0.3)
    (`KismetSystemLibrary.K2_ClearAndInvalidateTimerHandle` (`self.ToppleTimer`))
    (`self.DetachAndSimulate` (`self.Sphere`))
    (`self.DetachAndSimulate` (`self.Side2`))
    (`self.DetachAndSimulate` (`self.Side1`))
    (`self.DetachAndSimulate` (`self.Face1`))
    (`self.DetachAndSimulate` (`self.Face2`))
    (`self.DetachAndSimulate` (`self.Cylinder`))
    (`self.DetachAndSimulate` (`self.Top`))
    (`self.DetachAndSimulate` (`self.Bottom`))
    (`PrimitiveComponent.SetSimulatePhysics` (`self.CapsuleComponent`) false)
    (`PrimitiveComponent.SetCollisionEnabled` (`self.CapsuleComponent`) "NoCollision")
    (`/Engine/EditorBlueprintResources/StandardMacros.IsValid` _returnvalue
      (:`Is Valid`
        (`Controller.UnPossess` _returnvalue)))))

(fn `UserConstructionScript`
  (`parent.UserConstructionScript`))