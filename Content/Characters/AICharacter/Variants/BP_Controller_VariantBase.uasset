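; Base AI controller for AI character variants, managing behavior logic startup and shutdown.
; On BeginPlay it starts the brain component, initializes the base blackboard and increments its LivingAllies count.
; On UnPossess it stops the logic and destroys its spatial, pathing and perception components.
; A spatial position-choosing call with pathfinding remains in the graph but is disconnected.
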(event `self.ReceiveBeginPlay`
  (`parent.ReceiveBeginPlay`)
  (`BrainComponent.StartLogic` (`self.BrainComponent`))
  (bind _blackboardcomponent (`self.UseBlackboard` "/Game/Characters/AICharacter/Variants/BlackboardBase.BlackboardBase"))
  (`BlackboardComponent.SetValueAsInt` _blackboardcomponent (`self.Living Allies`) (+ (`BlackboardComponent.GetValueAsInt` _blackboardcomponent (`self.Living Allies`)) 1)))

(event `self.ReceiveTick`
  (params (DeltaSeconds :type "Float (single-precision)"))
  (`parent.ReceiveTick` DeltaSeconds))

(event `self.ReceiveUnPossess`
  (params (UnpossessedPawn :type "Pawn Object Reference"))
  (`BrainComponent.StopLogic` (`self.BrainComponent`) "")
  (`ActorComponent.K2_DestroyComponent` (`self.BP_SpatialComponent`))
  (`ActorComponent.K2_DestroyComponent` (`self.GAPathComponent`))
  (`ActorComponent.K2_DestroyComponent` (`self.GAPerception`)))

(fn `UserConstructionScript`
  (`parent.UserConstructionScript`))