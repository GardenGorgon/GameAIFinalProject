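; Fodder variant of the AI character, adding a low-health signal for its AI.
; When its VitalityComponent takes damage and HP is at or below 25, it sets the LowHealth key on the controller's Blackboard to true.
; This graph never clears that key, and a leftover LowHealthTrue assignment is unreachable.
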(event `self.VitalityComponent.Damaged`
  (bind _returnvalue (<= (`/Game/Characters/AICharacter/Variants/BP_VitalityComponent.HP` (`self.VitalityComponent`)) 25.0))
  (if _returnvalue
    (`BlackboardComponent.SetValueAsBool` (`AIBlueprintHelperLibrary.GetBlackboard` (`self.GetController`)) (`self.Low_Health`) _returnvalue)))

(fn `UserConstructionScript`
  (`parent.UserConstructionScript`))