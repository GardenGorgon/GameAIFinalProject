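; BP_VitalityComponent is a health component, filed under AI character variants, that tracks HP and death state.
; HP starts at MaxHP on BeginPlay, and each Damage event subtracts from it and calls Damaged.
; At zero or below, or through Kill, ExecuteDeath sets IsDead and calls Death.
; Damage does not check IsDead, so further hits after death call both again.
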(event `self.ReceiveBeginPlay`
  (set `self.HP` (`self.MaxHP`)))

(event `Damage`
  (params (Location :type "Vector Structure") (Vector :type "Vector Structure") (DamageAmount :type "Float (double-precision)"))
  (bind _output_get (set `self.HP` (- (`self.HP`) DamageAmount)))
  (`self.Damaged`)
  (if (<= _output_get 0.0)
    (`self.ExecuteDeath`)))

(event `ExecuteDeath`
  (set `self.IsDead` true)
  (`self.Death`))

(event `Kill`
  (set `self.HP` 0.0)
  (`self.ExecuteDeath`))